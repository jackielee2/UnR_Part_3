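; B_Bird is a sparrow actor that flies along +X at a random speed and drops when it overlaps B_Owl.
; Tick moves it, cycles its sprite animation through a dynamic material's Index parameter at a random rate, and projects its position to screen space.
; The first owl hit stops animation, rotates it, redirects movement downward and plays a sound.
; It destroys itself beyond the viewport's right or bottom edge plus a margin.
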(event `self.ReceiveBeginPlay`
  (`self.Get Screen Size`))

(event `self.ReceiveActorBeginOverlap`
  (params (OtherActor :type "Actor Object Reference"))
  ;[1 1 1] 충돌 이벤트 발생
  ;[1 1 1] 1) 충돌한 액터의 이름이 "B_Owl"인지 체크
  (if (`KismetStringLibrary.EqualEqual_StrStr` (`KismetSystemLibrary.GetDisplayName` OtherActor) "B_Owl")
    ;[1 1 1] 2) 충돌이 발생한 이후에도 충돌이 다시 발생할 수 있으므로 한번만 처리.
    (`/Engine/EditorBlueprintResources/StandardMacros.DoOnce` false
      (:`Completed`
        ;[1 1 1] 3) 참새 낙하 처리
        (`self.Drop Bird`)))))

(event `self.ReceiveTick`
  (params (DeltaSeconds :type "Float (single-precision)"))
  (`self.Move Bird`)
  (`self.Get Screen Pos`)
  (`self.Check Destroy`)
  (`self.Anim Bird`))

(fn `Anim Bird`
  (if (not (`self.Is Dead`))
    (bind _output_get (set `self.Anim Delay` (- (`self.Anim Delay`) (`GameplayStatics.GetWorldDeltaSeconds`))))
    (if (< _output_get 0.0)
      (set `self.Anim Delay` (/ 1.0 (`self.Anim Per Sec`)))
      (`self.Set Anim Index`))))

(fn `Check Destroy`
  ;[1 1 1] 2)  벗어난 경우에만 액터 제거..
  (if (or (> (`self.Pos X`) (`self.Screen Width`)) (> (`self.Pos Y`) (`self.Screen Height`)))
    (`self.K2_DestroyActor`)))

(fn `Drop Bird`
  ;[1 1 1] 1) 참새가 추락중임을 설정.
  (set `self.Is Dead` true)
  ;[1 1 1] 2) 참새가 화면의 아래쪽을 향하도록 Y축으로 180도 회전
  (`self.K2_SetActorRotation` (struct :`Pitch` 180.0))
  ;[1 1 1] 3) 참새의 이동방향을 화면 아래쪽으로 설정
  (set `self.Dir` (0.0 0.0 -1.0))
  ;[1 1 1] 4) 참새 사운드 효과 재생.
  (`GameplayStatics.PlaySoundAtLocation` "/Game/Audios/bird.bird" (`self.K2_GetActorLocation`) (struct) 1.0 1.0 0.0 null null null))

(fn `Get Screen Pos`
  (bind (_x _y) (`KismetMathLibrary.BreakVector2D` (`PlayerController.ProjectWorldLocationToScreen` (`GameplayStatics.GetPlayerController` 0) (`self.K2_GetActorLocation`) false)))
  ;[1 1 1] 2)  변환된 좌표를 각각 [ Pos X ], [ Pos Y ]에 저장..
  (set `self.Pos X` _x)
  (set `self.Pos Y` _y))

(fn `Get Screen Size`
  (bind (_sizex _sizey) (`PlayerController.GetViewportSize` (`GameplayStatics.GetPlayerController` 0)))
  ;[1 1 1] 2)  화면의 가로영역 경계 계산..
  (set `self.Screen Width` (`KismetMathLibrary.Conv_IntToDouble` (+ _sizex 50)))
  ;[1 1 1] 3)  화면의 세로영역 경계 계산..
  (set `self.Screen Height` (`KismetMathLibrary.Conv_IntToDouble` (+ _sizey 50))))

(fn `Init Bird`
  (bind _returnvalue (`KismetMathLibrary.RandomFloatInRange` 12.0 18.0))
  ;[1 1 1] 1)  초당 애니메이션 횟수를 12 ~ 18 회
  ;      사이로 랜덤 설정.
  (set `self.Anim Per Sec` _returnvalue)
  ;[1 1 1] 2)  애니메이션 간격 설정.
  ; 	  -  1 / 현재 설정된 애니메이션 횟수.
  (set `self.Anim Delay` (/ 1.0 _returnvalue))
  ;[1 1 1] 3)  300 ~ 600사이 값으로 이동 속도 설정
  (set `self.Speed` (`KismetMathLibrary.RandomFloatInRange` 300.0 600.0))
  (set `self.Dir` (1.0 0.0 0.0)) ; 4)  오른쪽으로 이동방향 설정..
)

(fn `Move Bird`
  ;[1 1 1] 3) 월드 좌표를 기준으로 현재 참새의 위치에 2) 결과를 누적
  (`self.K2_AddActorWorldOffset` (* (`self.Dir`) (* (`self.Speed`) (`GameplayStatics.GetWorldDeltaSeconds`)))))

(fn `Set Anim Index`
  ;[1 1 1] 1)  [ Set Anim Index ] 가 호출될 때 마다 [ Anim Index ]가 하나씩 증가..
  (bind _output_get (set `self.Anim Index` (+ (`self.Anim Index`) 1.0)))
  ;[1 1 1] 2)  참새 머터리얼( M_Bird )의 [ Index ] 에
  ;       [ Anim Index ]값 설정..
  (`MaterialInstanceDynamic.SetScalarParameterValue` (`self.Bird Instance`) "Index" _output_get))

(fn `UserConstructionScript`
  ;[1 1 1] 1)  [ Bird 컴포넌트 ] > [ 0번째 머터리얼 ] 인스턴스화..
  (bind _returnvalue (`PrimitiveComponent.CreateDynamicMaterialInstance` (`self.Bird`) 0 null "None"))
  (set `self.Bird Instance` _returnvalue) ; 2)  인스턴스화 된 정보를 참조..
  (`self.Init Bird`) ; 3)  참새 관련 정보 초기화..
)