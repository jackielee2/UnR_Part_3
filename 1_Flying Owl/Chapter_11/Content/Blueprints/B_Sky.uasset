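; B_Sky is the sky backdrop, camera view target and branch spawner for a vertical climbing game with an owl pawn.
; Construction applies the scroll speed to a dynamic sky material; BeginPlay takes over the view and spawns the first branch.
; SetCameraPos moves the actor to track a supplied maximum height.
; Tick spawns a resized B_Branch at random X whenever SpawnPoint rises far enough above the last branch.
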(event `self.ReceiveBeginPlay`
  (`PlayerController.SetViewTargetWithBlend` (`GameplayStatics.GetPlayerController` 0) self 0.0 "VTBlend_Linear" 0.0 false)
  (bind _asb_owl (cast `/Game/Blueprints/B_Owl` (`GameplayStatics.GetPlayerPawn` 0)))
  (`/Game/Blueprints/B_Owl.Get Screen Size` _asb_owl)
  (bind _returnvalue (`|SpawnActorFromClass` "/Game/Blueprints/B_Branch.B_Branch_C" (`SceneComponent.K2_GetComponentToWorld` (`self.Spawn Point`)) "Undefined" "OverrideRootScale" null null))
  (set `self.Last Branch` _returnvalue))

(event `self.ReceiveTick`
  (params (DeltaSeconds :type "Float (single-precision)"))
  (`self.Make New Branch`))

(fn `Check New Branch`
  (returns (`Can Branch` :type Boolean) (Location :type "Vector Structure"))
  (bind _returnvalue (> (.z (`SceneComponent.K2_GetComponentLocation` (`self.Spawn Point`))) (+ (.z (`self.K2_GetActorLocation` (`self.Last Branch`))) 300.0)))
  (if _returnvalue
    (bind _return_value (`self.Get Branch Location`)))
  (return _returnvalue _return_value))

(fn `Get Branch Location`
  (returns (`Return Value` :type "Vector Structure"))
  (return (`KismetMathLibrary.MakeVector` (`KismetMathLibrary.RandomFloatInRange` -250.0 250.0) (.y (`SceneComponent.K2_GetComponentLocation` (`self.Spawn Point`))) (.z (`SceneComponent.K2_GetComponentLocation` (`self.Spawn Point`))))))

(fn `Make New Branch`
  (bind (_can_branch _location) (`self.Check New Branch`))
  (if _can_branch
    (bind _returnvalue (`|SpawnActorFromClass` "/Game/Blueprints/B_Branch.B_Branch_C" (`KismetMathLibrary.Conv_VectorToTransform` _location) "Undefined" "OverrideRootScale" null null))
    (bind _output_get (set `self.Last Branch` _returnvalue))
    (`/Game/Blueprints/B_Branch.Set Branch Size` _output_get)))

(fn `Set Camera Pos`
  (params (`Max Height` :type "Float (double-precision)"))
  (`self.K2_SetActorLocation` (`KismetMathLibrary.MakeVector` 0.0 0.0 (- `Max Height` 320.0))))

(fn `UserConstructionScript`
  (bind _returnvalue (`PrimitiveComponent.CreateDynamicMaterialInstance` (`self.Sky`) 0 null "None"))
  (`MaterialInstanceDynamic.SetScalarParameterValue` _returnvalue "Speed" (`self.SkySpeed`)))