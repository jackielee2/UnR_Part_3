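; B_Owl is the player-controlled owl in a vertical jumping game, bouncing upward whenever a short downward trace hits a BRANCH-tagged actor.
; Tick applies manual gravity movement, swaps wing textures by vertical direction and feeds new peak height to B_Sky's camera.
; MoveRight input eases horizontal speed, blocks it at screen edges and flags death below the screen.
; Death stops movement and triggers game-over audio once; ShowMenu is an empty stub.
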(event `self.ReceiveBeginPlay`
  (bind _outactors (`GameplayStatics.GetAllActorsOfClass` "/Game/Blueprints/B_Sky.B_Sky_C"))
  (set `self.Sky` (`|GetArrayItem` _outactors))
  (`AudioComponent.Play` (`self.BGM`) 0.0))

(event `self.ReceiveTick`
  (params (DeltaSeconds :type "Float (single-precision)"))
  (if (`self.Is Dead`)
    (`/Engine/EditorBlueprintResources/StandardMacros.DoOnce` false
      (:`Completed`
        (`self.Set Game Over`)))
    (else
      (`self.Check Branch`)
      (`self.Move Owl`)
      (`self.Set Max Height`)
      (`self.Set Wing`))))

(event `InputAxis|MoveRight`
  (params (AxisValue :type "Float (single-precision)"))
  (`self.Line Interp` AxisValue)
  (`self.Get Screen Size`))

(fn `Check Branch`
  (bind _returnvalue (`self.K2_GetActorLocation`))
  (bind (_outhit _returnvalue_2) (`KismetSystemLibrary.LineTraceSingle` :`Start` _returnvalue :`End` (+ _returnvalue (0.0 0.0 -40.0)) :`TraceChannel` "TraceTypeQuery3" :`DrawDebugType` "ForOneFrame"))
  (if _returnvalue_2
    (if (`self.ActorHasTag` (`.HitActor` (`GameplayStatics.BreakHitResult` _outhit)) "BRANCH")
      (`self.Jump Owl`))))

(fn `Check Screen Limit`
  (bind _axis (`self.Axis`))
  (bind _screen_x (`self.Screen X`))
  (`self.Get Screen Pos`)
  (if (or (and (< _axis 0.0) (< _screen_x 80.0)) (and (> _axis 0.0) (> _screen_x (- (`self.Screen Width`) 80.0))))
    (set `self.Dir X` 0.0)))

(fn `Get Screen Pos`
  (bind (_x _y) (`KismetMathLibrary.BreakVector2D` (`PlayerController.ProjectWorldLocationToScreen` (`GameplayStatics.GetPlayerController` 0) (`self.K2_GetActorLocation`) false)))
  (set `self.Screen X` _x)
  (bind _output_get (set `self.Screen Y` _y))
  (set `self.Is Dead` (> _output_get (+ (`self.Screen Height`) 80.0))))

(fn `Get Screen Size`
  (bind (_sizex _sizey) (`PlayerController.GetViewportSize` (`GameplayStatics.GetPlayerController` 0)))
  (set `self.Screen Width` (`KismetMathLibrary.Conv_IntToDouble` _sizex))
  (set `self.Screen Height` (`KismetMathLibrary.Conv_IntToDouble` _sizey)))

(fn `Jump Owl`
  (set `self.Dir Z` (`self.Speed Jump`))
  (`AudioComponent.Play` (`self.Jump Sound`) 0.01))

(fn `Line Interp`
  (params (`Axis Value` :type "Float (double-precision)"))
  (bind _output_get (set `self.Axis` `Axis Value`))
  (set `self.Dir X` (`KismetMathLibrary.FInterpTo` (`self.Dir X`) (* _output_get (`self.Speed Jump`)) (`GameplayStatics.GetWorldDeltaSeconds`) (`self.Speed Move`)))
  (`self.Check Screen Limit`))

(fn `Move Owl`
  (bind _output_get (set `self.Dir Z` (- (`self.Dir Z`) (* (`self.Gravity`) (`GameplayStatics.GetWorldDeltaSeconds`)))))
  (`self.K2_AddActorLocalOffset` (* (`KismetMathLibrary.MakeVector` (`self.Dir X`) 0.0 _output_get) (`GameplayStatics.GetWorldDeltaSeconds`))))

(fn `Set Game Over`
  (`AudioComponent.Stop` (`self.BGM`))
  (`AudioComponent.Play` (`self.Snd Game Over`) 0.0)
  (`self.Show Menu`))

(fn `Set Max Height`
  (bind _z (.z (`self.K2_GetActorLocation`)))
  (if (> _z (`self.Max Height`))
    (bind _output_get (set `self.Max Height` _z))
    (`/Game/Blueprints/B_Sky.Set Camera Pos` (`self.Sky`) _output_get)))

(fn `Set Wing`
  (bind _instance_owl (`self.Instance Owl`))
  (if (> (`self.Dir Z`) 0.0)
    (`MaterialInstanceDynamic.SetTextureParameterValue` _instance_owl "OwlImage" "/Game/Textures/owl1.owl1")
    (else
      (`MaterialInstanceDynamic.SetTextureParameterValue` _instance_owl "OwlImage" "/Game/Textures/owl2.owl2"))))

(fn `Show Menu`)

(fn `UserConstructionScript`
  (bind _returnvalue (`PrimitiveComponent.CreateDynamicMaterialInstance` (`self.Owl`) 0 "/Game/Materials/M_Owl.M_Owl" "None"))
  (set `self.Instance Owl` _returnvalue))