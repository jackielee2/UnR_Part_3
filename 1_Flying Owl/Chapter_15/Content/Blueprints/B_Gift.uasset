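; B_Gift is a gift pickup actor that plays the Gift sound and destroys itself when an overlapping actor's display name is "B_Owl".
; The construction script creates a dynamic instance of M_Gift and randomly sets one of three gift textures on it.
; Each Tick, it projects its location to screen space and destroys itself once it is slightly below the bottom of the viewport.
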(event `self.ReceiveActorBeginOverlap`
  (params (OtherActor :type "Actor Object Reference"))
  ;[1 1 1] 2) 1) 의 결과가 맞다면 gift.wav 사운드 연출
  (if (`KismetStringLibrary.EqualEqual_StrStr` (`KismetSystemLibrary.GetDisplayName` OtherActor) "B_Owl")
    (`GameplayStatics.PlaySoundAtLocation` "/Game/Audios/gift.gift" (`self.K2_GetActorLocation`) (struct) 1.0 1.0 0.0 null null null)
    (`self.K2_DestroyActor`)))

(event `self.ReceiveTick`
  (params (DeltaSeconds :type "Float (single-precision)"))
  (`self.Check Position`))

(fn `Check Position`
  (bind _returnvalue (`GameplayStatics.GetPlayerController` 0))
  ;[1 1 1] 3) 화면의 높이 + 50 보다 더 아래로 선물이 위치해있는지 확인한뒤 선물을 제거한다.
  (if (> (`.Y` (`KismetMathLibrary.BreakVector2D` (`PlayerController.ProjectWorldLocationToScreen` _returnvalue (`self.K2_GetActorLocation`) false))) (`KismetMathLibrary.Conv_IntToDouble` (+ (`.SizeY` (`PlayerController.GetViewportSize` _returnvalue)) 50)))
    (`self.K2_DestroyActor`)))

(fn `Set Gift Image`
  (bind _gift_instance (`self.Gift Instance`))
  ;[1 1 1] 2) 1)의 결과를 Gift Num으로 설정
  (bind _output_get (set `self.Gift Num` (`KismetMathLibrary.RandomIntegerInRange` 1 3)))
  ;[1 1 1] 3) 2)의 결과에 따라 분기
  (switch `int` _output_get ; Start Index : 1 / Has Default Pin : false
    (:`1`
      ;[1 1 1] 4) 머터리얼 인스턴스 변수를 이용하여 머터리얼의 파라미터로 이미지 설정
      (`MaterialInstanceDynamic.SetTextureParameterValue` _gift_instance "Gift Image" "/Game/Textures/gift1.gift1"))
    (:`2`
      (`MaterialInstanceDynamic.SetTextureParameterValue` _gift_instance "Gift Image" "/Game/Textures/gift2.gift2"))
    (:`3`
      (`MaterialInstanceDynamic.SetTextureParameterValue` _gift_instance "Gift Image" "/Game/Textures/gift3.gift3"))))

(fn `UserConstructionScript`
  ;[1 1 1] Source Material : M_Gift
  (bind _returnvalue (`PrimitiveComponent.CreateDynamicMaterialInstance` (`self.Gift`) 0 "/Game/Materials/M_Gift.M_Gift" "None"))
  (set `self.Gift Instance` _returnvalue)
  (`self.Set Gift Image`))