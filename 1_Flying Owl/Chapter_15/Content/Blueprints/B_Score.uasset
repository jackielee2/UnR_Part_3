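; B_Score is a score text actor meant to rise, change alpha and then destroy itself.
; The construction script creates a dynamic material instance on the Score text, and SetScore formats the number with digit grouping and applies a color.
; The TextRender timeline drives the material's Alpha and upward movement, destroying the actor on finish.
; No wire in the graph starts that timeline, and the test SetScore call is disconnected.
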(event `self.ReceiveBeginPlay`)

(fn `Set Score`
  (params (Score :type Integer) (Color :type "LinearColor Structure"))
  (bind _score (`self.Score`))
  ;[1 1 1] 1) 매개변수 설정 - Score, Color
  (`TextRenderComponent.K2_SetText` _score (`|FormatText` "{Currency}" (`KismetTextLibrary.Conv_IntToText` Score))) ; 문자열 설정
  (`TextRenderComponent.SetTextRenderColor` _score (`KismetMathLibrary.Conv_LinearColorToColor` Color)) ; 색깔 설정
)

(fn `UserConstructionScript`
  (bind _returnvalue (`PrimitiveComponent.CreateDynamicMaterialInstance` (`self.Score`) 0 null "None"))
  (set `self.Font Instance` _returnvalue))