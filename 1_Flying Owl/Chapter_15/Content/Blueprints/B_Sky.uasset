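; Sky backdrop actor that serves as the player's camera view and spawns the objects of a vertical climbing level with B_Owl.
; SetCameraPos moves the actor to follow a given max height, carrying SpawnPoint with it.
; Each Tick, it adds a randomly placed branch once SpawnPoint clears the last one, and randomly spawns birds and a capped number of gifts.
; The construction script sets the sky material's scroll speed through a dynamic instance.
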(event `self.ReceiveBeginPlay`
  (`PlayerController.SetViewTargetWithBlend` (`GameplayStatics.GetPlayerController` 0) self 0.0 "VTBlend_Linear" 0.0 false)
  (bind _asb_owl (cast `/Game/Blueprints/B_Owl` (`GameplayStatics.GetPlayerPawn` 0)))
  (`/Game/Blueprints/B_Owl.Get Screen Size` _asb_owl)
  (bind _returnvalue (`|SpawnActorFromClass` "/Game/Blueprints/B_Branch.B_Branch_C" (`SceneComponent.K2_GetComponentToWorld` (`self.Spawn Point`)) "Undefined" "OverrideRootScale" null null))
  (set `self.Last Branch` _returnvalue))

(event `self.ReceiveTick`
  (params (DeltaSeconds :type "Float (single-precision)"))
  (`self.Make New Branch`)
  (`self.Make Bird`)
  (`self.Make Gift`))

(fn `Check New Branch`
  (returns (`Can Branch` :type Boolean) (Location :type "Vector Structure"))
  (bind _returnvalue (> (.z (`SceneComponent.K2_GetComponentLocation` (`self.Spawn Point`))) (+ (.z (`self.K2_GetActorLocation` (`self.Last Branch`))) 300.0)))
  (if _returnvalue
    (bind _return_value (`self.Get Branch Location`)))
  (return _returnvalue _return_value))

(fn `Get Branch Location`
  (returns (`Return Value` :type "Vector Structure"))
  (return (`KismetMathLibrary.MakeVector` (`KismetMathLibrary.RandomFloatInRange` -250.0 250.0) (.y (`SceneComponent.K2_GetComponentLocation` (`self.Spawn Point`))) (.z (`SceneComponent.K2_GetComponentLocation` (`self.Spawn Point`))))))

(fn `Get Gift Count`
  (returns (`Return Value` :type Integer))
  ;[1 1 1] 1) 씬에 등록된 액터 중 B_Gift 클래스 액터를 찾아 배열에 저장.
  (bind _outactors (`GameplayStatics.GetAllActorsOfClass` "/Game/Blueprints/B_Gift.B_Gift_C"))
  ;[1 1 1] 2) 배열의 길이를 반환
  (return (`KismetArrayLibrary.Array_Length` _outactors)))

(fn `Make Bird`
  (if (> (`KismetMathLibrary.RandomFloatInRange` 0.0 1000.0) 990.0)
    ;[1 1 1] 3) 2)의 좌표값으로 참새 액터를 만들고 Tick 이벤트에 추가.
    (`|SpawnActorFromClass` "/Game/Blueprints/B_Bird.B_Bird_C" (`KismetMathLibrary.Conv_VectorToTransform` (`KismetMathLibrary.MakeVector` -1100.0 -5.0 (+ (.z (`SceneComponent.K2_GetComponentLocation` (`self.Spawn Point`))) (`KismetMathLibrary.RandomFloatInRange` -50.0 50.0)))) "Undefined" "OverrideRootScale" null null) ; [ Spawn Actor from Class ]로 검색
  ))

(fn `Make Gift`
  ;[1 1 1] 1) 현재 생성되어 있는 선물의 갯수를 파악하여 5개를 넘지 않으면 계속 진행.
  (bind _return_value (`self.Get Gift Count`))
  (if (< _return_value 5)
    ;[1 1 1] 2) 10 / 1000의 확률 체크
    (if (> (`KismetMathLibrary.RandomFloatInRange` 0.0 1000.0) 990.0)
      ;[1 1 1] 5) 4)의 위치값을 이용하여 B_Gift 클래스 액터를 생성한 뒤 Tick 이벤트에 추가.
      (`|SpawnActorFromClass` "/Game/Blueprints/B_Gift.B_Gift_C" (`KismetMathLibrary.Conv_VectorToTransform` (`KismetMathLibrary.MakeVector` (`KismetMathLibrary.RandomFloatInRange` -500.0 500.0) -10.0 (+ (.z (`SceneComponent.K2_GetComponentLocation` (`self.Spawn Point`))) (`KismetMathLibrary.RandomFloatInRange` 50.0 150.0)))) "Undefined" "OverrideRootScale" null null))))

(fn `Make New Branch`
  (bind (_can_branch _location) (`self.Check New Branch`))
  (if _can_branch
    (bind _returnvalue (`|SpawnActorFromClass` "/Game/Blueprints/B_Branch.B_Branch_C" (`KismetMathLibrary.Conv_VectorToTransform` _location) "Undefined" "OverrideRootScale" null null))
    (bind _output_get (set `self.Last Branch` _returnvalue))
    (`/Game/Blueprints/B_Branch.Set Branch Size` _output_get)))

(fn `Set Camera Pos`
  (params (`Max Height` :type "Float (double-precision)"))
  (`self.K2_SetActorLocation` (`KismetMathLibrary.MakeVector` 0.0 0.0 (- `Max Height` 320.0))))

(fn `UserConstructionScript`
  (bind _returnvalue (`PrimitiveComponent.CreateDynamicMaterialInstance` (`self.Sky`) 0 null "None"))
  (`MaterialInstanceDynamic.SetScalarParameterValue` _returnvalue "Speed" (`self.SkySpeed`)))