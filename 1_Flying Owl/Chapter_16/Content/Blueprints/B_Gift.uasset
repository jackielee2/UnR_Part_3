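; B_Gift is a collectible gift actor that awards points when the owl touches it.
; Its construction script randomly picks one of three gift textures on a dynamic material instance, and that index scales the score.
; An overlap, matched by display name "B_Owl", plays a sound, spawns a B_Score popup, updates the player owl's gift totals and destroys the gift.
; Tick destroys gifts that drop below the screen's bottom edge, using screen-space projection.
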(event `self.ReceiveActorBeginOverlap`
  (params (OtherActor :type "Actor Object Reference"))
  ;[1 1 1] 2) 1) 의 결과가 맞다면 gift.wav 사운드 연출
  (if (`KismetStringLibrary.EqualEqual_StrStr` (`KismetSystemLibrary.GetDisplayName` OtherActor) "B_Owl")
    (`GameplayStatics.PlaySoundAtLocation` "/Game/Audios/gift.gift" (`self.K2_GetActorLocation`) (struct) 1.0 1.0 0.0 null null null)
    (`self.Set Score Text`)
    (`self.K2_DestroyActor`)))

(event `self.ReceiveTick`
  (params (DeltaSeconds :type "Float (single-precision)"))
  (`self.Check Position`))

(fn `Check Position`
  (bind _returnvalue (`GameplayStatics.GetPlayerController` 0))
  ;[1 1 1] 3) 화면의 높이 + 50 보다 더 아래로 선물이 위치해있는지 확인한뒤 선물을 제거한다.
  (if (> (`.Y` (`KismetMathLibrary.BreakVector2D` (`PlayerController.ProjectWorldLocationToScreen` _returnvalue (`self.K2_GetActorLocation`) false))) (`KismetMathLibrary.Conv_IntToDouble` (+ (`.SizeY` (`PlayerController.GetViewportSize` _returnvalue)) 50)))
    (`self.K2_DestroyActor`)))

(fn `Set Gift Image`
  (bind _gift_instance (`self.Gift Instance`))
  ;[1 1 1] 2) 1)의 결과를 Gift Num으로 설정
  (bind _output_get (set `self.Gift Num` (`KismetMathLibrary.RandomIntegerInRange` 1 3)))
  ;[1 1 1] 3) 2)의 결과에 따라 분기
  (switch `int` _output_get ; Start Index : 1 / Has Default Pin : false
    (:`1`
      ;[1 1 1] 4) 머터리얼 인스턴스 변수를 이용하여 머터리얼의 파라미터로 이미지 설정
      (`MaterialInstanceDynamic.SetTextureParameterValue` _gift_instance "Gift Image" "/Game/Textures/gift1.gift1"))
    (:`2`
      (`MaterialInstanceDynamic.SetTextureParameterValue` _gift_instance "Gift Image" "/Game/Textures/gift2.gift2"))
    (:`3`
      (`MaterialInstanceDynamic.SetTextureParameterValue` _gift_instance "Gift Image" "/Game/Textures/gift3.gift3"))))

(fn `Set Owl Score`
  ;[1 1 1] 1) 올빼미 액터 정보를 참조
  (bind _asb_owl (cast `/Game/Blueprints/B_Owl` (`GameplayStatics.GetPlayerPawn` 0)))
  ;[1 1 1] 2) 선물 카운트를 하나 증가
  (`/Engine/EditorBlueprintResources/StandardMacros.IncrementInt` (`/Game/Blueprints/B_Owl.Count Gift` _asb_owl)
    (:`  `
      ;[1 1 1] 3) 선물의 번호에 따른 점수를 올빼미의 선물 총점 관리 변수에 누적
      (set `/Game/Blueprints/B_Owl.Gift Score` (+ (`/Game/Blueprints/B_Owl.Gift Score` _asb_owl) (* (`self.Gift Num`) 500)) _asb_owl))))

(fn `Set Score Text`
  ;[1 1 1] 1) 선물의 위치값을 이용하여 [ B_Score ] 액터 생성
  (bind _returnvalue (`|SpawnActorFromClass` "/Game/Blueprints/B_Score.B_Score_C" (`self.GetTransform`) "Undefined" "OverrideRootScale" null null))
  ;[1 1 1] 2) 선물의 인덱스로 점수를 설정
  (`/Game/Blueprints/B_Score.Set Score` _returnvalue (* (`self.Gift Num`) 500) (struct :`R` 0.360444 :`G` 0.692708 :`B` 0.310821 :`A` 1.0))
  (`self.Set Owl Score`))

(fn `UserConstructionScript`
  ;[1 1 1] Source Material : M_Gift
  (bind _returnvalue (`PrimitiveComponent.CreateDynamicMaterialInstance` (`self.Gift`) 0 "/Game/Materials/M_Gift.M_Gift" "None"))
  (set `self.Gift Instance` _returnvalue)
  (`self.Set Gift Image`))