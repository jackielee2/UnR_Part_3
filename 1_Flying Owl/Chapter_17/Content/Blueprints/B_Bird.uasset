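; Sparrow actor that flies along +X at a random speed and costs the player points when the owl hits it.
; Each tick moves it, advances a flipbook animation through a dynamic material's Index parameter, and destroys it past the screen's right or bottom edge using projected screen position.
; The first B_Owl overlap spawns a red negative B_Score, increments the owl's CountBird, then flips the bird, plays a sound and sends it falling.
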(event `self.ReceiveBeginPlay`
  (`self.Get Screen Size`))

(event `self.ReceiveActorBeginOverlap`
  (params (OtherActor :type "Actor Object Reference"))
  ;[1 1 1] 충돌 이벤트 발생
  ;[1 1 1] 1) 충돌한 액터의 이름이 "B_Owl"인지 체크
  (if (`KismetStringLibrary.EqualEqual_StrStr` (`KismetSystemLibrary.GetDisplayName` OtherActor) "B_Owl")
    ;[1 1 1] 2) 충돌이 발생한 이후에도 충돌이 다시 발생할 수 있으므로 한번만 처리.
    (`/Engine/EditorBlueprintResources/StandardMacros.DoOnce` false
      (:`Completed`
        ;[1 1 1] 4) 점수 처리
        (`self.Set Score Text`)
        ;[1 1 1] 3) 참새 낙하 처리
        (`self.Drop Bird`)))))

(event `self.ReceiveTick`
  (params (DeltaSeconds :type "Float (single-precision)"))
  (`self.Move Bird`)
  (`self.Get Screen Pos`)
  (`self.Check Destroy`)
  (`self.Anim Bird`))

(fn `Anim Bird`
  (if (not (`self.Is Dead`))
    (bind _output_get (set `self.Anim Delay` (- (`self.Anim Delay`) (`GameplayStatics.GetWorldDeltaSeconds`))))
    (if (< _output_get 0.0)
      (set `self.Anim Delay` (/ 1.0 (`self.Anim Per Sec`)))
      (`self.Set Anim Index`))))

(fn `Check Destroy`
  (if (or (> (`self.Pos X`) (`self.Screen Width`)) (> (`self.Pos Y`) (`self.Screen Height`)))
    (`self.K2_DestroyActor`)))

(fn `Drop Bird`
  ;[1 1 1] 1) 참새가 추락중임을 설정.
  (set `self.Is Dead` true)
  ;[1 1 1] 2) 참새가 화면의 아래쪽을 향하도록 Y축으로 180도 회전
  (`self.K2_SetActorRotation` (struct :`Pitch` 180.0))
  ;[1 1 1] 3) 참새의 이동방향을 화면 아래쪽으로 설정
  (set `self.Dir` (0.0 0.0 -1.0))
  ;[1 1 1] 4) 참새 사운드 효과 재생.
  (`GameplayStatics.PlaySoundAtLocation` "/Game/Audios/bird.bird" (`self.K2_GetActorLocation`) (struct) 1.0 1.0 0.0 null null null))

(fn `Get Screen Pos`
  (bind (_x _y) (`KismetMathLibrary.BreakVector2D` (`PlayerController.ProjectWorldLocationToScreen` (`GameplayStatics.GetPlayerController` 0) (`self.K2_GetActorLocation`) false)))
  (set `self.Pos X` _x)
  (set `self.Pos Y` _y))

(fn `Get Screen Size`
  (bind (_sizex _sizey) (`PlayerController.GetViewportSize` (`GameplayStatics.GetPlayerController` 0)))
  (set `self.Screen Width` (`KismetMathLibrary.Conv_IntToDouble` (+ _sizex 50)))
  (set `self.Screen Height` (`KismetMathLibrary.Conv_IntToDouble` (+ _sizey 50))))

(fn `Init Bird`
  (bind _returnvalue (`KismetMathLibrary.RandomFloatInRange` 12.0 18.0))
  (set `self.Anim Per Sec` _returnvalue)
  (set `self.Anim Delay` (/ 1.0 _returnvalue))
  (set `self.Speed` (`KismetMathLibrary.RandomFloatInRange` 300.0 600.0))
  (set `self.Dir` (1.0 0.0 0.0)))

(fn `Move Bird`
  ;[1 1 1] 3) 월드 좌표를 기준으로 현재 참새의 위치에 2) 결과를 누적
  (`self.K2_AddActorWorldOffset` (* (`self.Dir`) (* (`self.Speed`) (`GameplayStatics.GetWorldDeltaSeconds`)))))

(fn `Set Anim Index`
  (bind _output_get (set `self.Anim Index` (+ (`self.Anim Index`) 1.0)))
  (`MaterialInstanceDynamic.SetScalarParameterValue` (`self.Bird Instance`) "Index" _output_get))

(fn `Set Score Text`
  ;[1 1 1] 1) [ B_Score ] 액터 생성
  (bind _returnvalue (`|SpawnActorFromClass` "/Game/Blueprints/B_Score.B_Score_C" (`self.GetTransform`) "Undefined" "OverrideRootScale" null null)) ; Class : B_Score / Spawn Transform : 현재 참새 트랜스롬 정보
  ;[1 1 1] 2) 액터로부터 [ B_Score ] 블프 클래스를 참조
  (bind _asb_score (cast `/Game/Blueprints/B_Score` _returnvalue))
  ;[1 1 1] 3) [ B_Score ] > [ Set Score  ] 함수를 이용하여 정보 설정.
  (`/Game/Blueprints/B_Score.Set Score` _asb_score -1000 (struct :`R` 1.0 :`A` 1.0))
  ;[1 1 1] 5] Pawn으로부터 올빼미 정보를 얻어온다
  (bind _asb_owl (cast `/Game/Blueprints/B_Owl` (`GameplayStatics.GetPlayerPawn` 0)))
  ;[1 1 1] 6] 올빼미의 [ Count Bird ] 횟수를 1 증가시킨다
  (`/Engine/EditorBlueprintResources/StandardMacros.IncrementInt` (`/Game/Blueprints/B_Owl.Count Bird` _asb_owl)))

(fn `UserConstructionScript`
  (bind _returnvalue (`PrimitiveComponent.CreateDynamicMaterialInstance` (`self.Bird`) 0 "/Game/Materials/M_Bird.M_Bird" "None"))
  (set `self.Bird Instance` _returnvalue)
  (`self.Init Bird`))