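; B_Branch is a branch actor tagged BRANCH that varies its look and size on spawn and removes itself once off-screen.
; Construction creates a dynamic M_Branch material; BeginPlay randomly picks its X and Y tiling from a parameter array and randomizes the actor's X scale.
; Every Tick projects the actor's location to screen space and destroys it once it passes slightly below the viewport's bottom edge.
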(event `self.ReceiveBeginPlay`
  (`self.Set Branch Image`)
  (`self.Set Branch Size`))

(event `self.ReceiveTick`
  (params (DeltaSeconds :type "Float (single-precision)"))
  (`self.Check Destroy`))

(fn `Check Destroy`
  (bind _returnvalue (`GameplayStatics.GetPlayerController` 0))
  (if (> (`.Y` (`KismetMathLibrary.BreakVector2D` (`PlayerController.ProjectWorldLocationToScreen` _returnvalue (`self.K2_GetActorLocation`) false))) (`KismetMathLibrary.Conv_IntToDouble` (+ (`.SizeY` (`PlayerController.GetViewportSize` _returnvalue)) 30)))
    (`self.K2_DestroyActor`)))

(fn `Set Branch Image`
  (bind _instance_branch (`self.Instance Branch`))
  (`MaterialInstanceDynamic.SetScalarParameterValue` _instance_branch "TilingX" (`|GetArrayItem` (`self.Param Array`) (`KismetMathLibrary.RandomIntegerInRange` 0 1)))
  (`MaterialInstanceDynamic.SetScalarParameterValue` _instance_branch "TilingY" (`|GetArrayItem` (`self.Param Array`) (`KismetMathLibrary.RandomIntegerInRange` 0 1))))

(fn `Set Branch Size`
  (`self.SetActorScale3D` (`KismetMathLibrary.MakeVector` (`KismetMathLibrary.RandomFloatInRange` 0.3 1.0) 1.0 1.0)))

(fn `UserConstructionScript`
  (bind _returnvalue (`PrimitiveComponent.CreateDynamicMaterialInstance` (`self.Branch`) 0 "/Game/Materials/M_Branch.M_Branch" "None"))
  (set `self.Instance Branch` _returnvalue)
  (set `self.Tags` (`|MakeArray` "BRANCH" :!type "Name")))