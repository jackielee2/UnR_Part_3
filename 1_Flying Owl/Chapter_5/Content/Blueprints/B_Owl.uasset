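; B_Owl is an owl Blueprint that moves along its local X axis from the MoveRight input axis.
; Each axis event eases Dirx toward input times SpeedMove and delta time with FInterpTo, giving acceleration and deceleration.
; The offset re-evaluates that interpolation on the updated Dirx and moves the actor without sweep.
; It also prints the axis value; all other events and the construction script are empty.
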(event `InputAxis|MoveRight`
  (params (AxisValue :type "Float (single-precision)"))
  (bind _returnvalue (`KismetMathLibrary.FInterpTo` (`self.Dirx`) (* AxisValue (`self.SpeedMove`) (`GameplayStatics.GetWorldDeltaSeconds`)) (`GameplayStatics.GetWorldDeltaSeconds`) 6.0))
  (`KismetSystemLibrary.PrintString` (`KismetStringLibrary.Conv_DoubleToString` AxisValue))
  (set `self.Dirx` _returnvalue)
  (`self.K2_AddActorLocalOffset` (`KismetMathLibrary.MakeVector` _returnvalue)))

(fn `UserConstructionScript`)