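; B_Branch is a branch actor that randomizes its look each time it begins play.
; The construction script creates a dynamic instance of M_Branch on the Branch component and tags the actor "BRANCH".
; On BeginPlay it sets the TilingX and TilingY material parameters to random picks from ParamArray, varying the image, then randomizes the actor's X scale to vary its size.
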(event `self.ReceiveBeginPlay`
  (`self.Set Branch Image`)
  (`self.Set Branch Size`))

(fn `Set Branch Image`
  (bind _instance_branch (`self.Instance Branch`))
  (`MaterialInstanceDynamic.SetScalarParameterValue` _instance_branch "TilingX" (`|GetArrayItem` (`self.Param Array`) (`KismetMathLibrary.RandomIntegerInRange` 0 1)))
  (`MaterialInstanceDynamic.SetScalarParameterValue` _instance_branch "TilingY" (`|GetArrayItem` (`self.Param Array`) (`KismetMathLibrary.RandomIntegerInRange` 0 1))))

(fn `Set Branch Size`
  (`self.SetActorScale3D` (`KismetMathLibrary.MakeVector` (`KismetMathLibrary.RandomFloatInRange` 0.3 1.0) 1.0 1.0)))

(fn `UserConstructionScript`
  (bind _returnvalue (`PrimitiveComponent.CreateDynamicMaterialInstance` (`self.Branch`) 0 "/Game/Materials/M_Branch.M_Branch" "None"))
  (set `self.Instance Branch` _returnvalue)
  (set `self.Tags` (`|MakeArray` "BRANCH" :!type "Name")))