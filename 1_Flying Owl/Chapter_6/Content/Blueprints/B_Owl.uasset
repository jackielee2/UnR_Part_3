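; B_Owl is the player owl pawn for a vertical branch-jumping game.
; The MoveRight axis moves it along local X with interpolated, frame-time-scaled speed.
; Helper functions trace downward for BRANCH-tagged actors to trigger a jump speed and sound, cache viewport size and screen position, and record maximum height.
; The event graph calls none of these helpers, and DirZ is set but never applied here.
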(event `InputAxis|MoveRight`
  (params (AxisValue :type "Float (single-precision)"))
  (bind _returnvalue (`KismetMathLibrary.FInterpTo` (`self.Dir X`) (* AxisValue (`self.Speed Move`) (`GameplayStatics.GetWorldDeltaSeconds`)) (`GameplayStatics.GetWorldDeltaSeconds`) 6.0))
  (set `self.Dir X` _returnvalue)
  (`self.K2_AddActorLocalOffset` (`KismetMathLibrary.MakeVector` _returnvalue)))

(fn `Check Branch`
  (bind _returnvalue (`self.K2_GetActorLocation`))
  (bind (_outhit _returnvalue_2) (`KismetSystemLibrary.LineTraceSingle` :`Start` _returnvalue :`End` (+ _returnvalue (0.0 0.0 -40.0)) :`TraceChannel` "TraceTypeQuery3" :`DrawDebugType` "ForOneFrame")) ; -  [ Start ] ~ [ End ] 로 가상의 선을 발사하여\n      충돌한 액터의 정보를 [ Out Hit ]으로 전달.\n\n    -  [ Trace Channel ] : [ Trigger ]\n    -  [ Draw Debug Type ] : [ For One Frame ]\n        [ Trace Color ] : [ Red ]\n        [ Trace Color ] : [ Green ]\n        [ Draw Time ] : [ 5 ]
  ;[1 1 1] [ 라인 트레이싱 ] 결과
  ; 1) 액터에 충돌했고
  ; 2) 액터의 태그가 BRANCH 라면...
  (if _returnvalue_2
    (if (`self.ActorHasTag` (`.HitActor` (`GameplayStatics.BreakHitResult` _outhit)) "BRANCH")
      (`self.Jump Owl`))))

(fn `Get Screen Pos`
  (bind (_x _y) (`KismetMathLibrary.BreakVector2D` (`PlayerController.ProjectWorldLocationToScreen` (`GameplayStatics.GetPlayerController` 0) (`self.K2_GetActorLocation`) false)))
  (set `self.Screen X` _x)
  (set `self.Screen Y` _y))

(fn `Get Screen Size`
  (bind (_sizex _sizey) (`PlayerController.GetViewportSize` (`GameplayStatics.GetPlayerController` 0)))
  (set `self.Screen Width` (`KismetMathLibrary.Conv_IntToDouble` _sizex))
  (set `self.Screen Height` (`KismetMathLibrary.Conv_IntToDouble` _sizey))
  (`KismetSystemLibrary.PrintString` "Get Screen Size 호출!!!"))

(fn `Jump Owl`
  (set `self.Dir Z` (`self.Speed Jump`))
  (`GameplayStatics.PlaySoundAtLocation` "/Game/Audios/jump.jump" (`self.K2_GetActorLocation`) (struct) 1.0 1.0 0.0 null null null) ; -  [ Sound 핀 ] : [ jump.wav ]
)

(fn `Set Max Height`
  (bind _z (.z (`self.K2_GetActorLocation`)))
  ;[1 1 1] - 현재 폰의 위치값중 높이( z ) 값만 추출후
  ;   최고 높이 값( Max Height )보다 크면 최고 높이 값을 갱신..
  (if (> _z (`self.Max Height`))
    (set `self.Max Height` _z)))

(fn `UserConstructionScript`)