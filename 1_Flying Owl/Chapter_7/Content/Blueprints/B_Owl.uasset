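; B_Owl is a player-controlled owl for a vertical branch-jumping game, currently wired only for smoothed horizontal movement from the MoveRight axis.
; Helper functions define manual gravity movement, a downward trace that jumps with sound off "BRANCH"-tagged actors, max-height tracking, and screen-projected edge limits that zero horizontal speed.
; The event graph calls none of these helpers, instead interpolating and applying the X offset inline.
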(event `InputAxis|MoveRight`
  (params (AxisValue :type "Float (single-precision)"))
  (bind _returnvalue (`KismetMathLibrary.FInterpTo` (`self.Dir X`) (* AxisValue (`self.Speed Move`) (`GameplayStatics.GetWorldDeltaSeconds`)) (`GameplayStatics.GetWorldDeltaSeconds`) 6.0))
  (set `self.Dir X` _returnvalue)
  (`self.K2_AddActorLocalOffset` (`KismetMathLibrary.MakeVector` _returnvalue)))

(fn `Check Branch`
  (bind _returnvalue (`self.K2_GetActorLocation`))
  (bind (_outhit _returnvalue_2) (`KismetSystemLibrary.LineTraceSingle` :`Start` _returnvalue :`End` (+ _returnvalue (0.0 0.0 -40.0)) :`TraceChannel` "TraceTypeQuery3" :`DrawDebugType` "ForOneFrame"))
  (if _returnvalue_2
    (if (`self.ActorHasTag` (`.HitActor` (`GameplayStatics.BreakHitResult` _outhit)) "BRANCH")
      (`self.Jump Owl`))))

(fn `Check Screen Limit`
  (bind _axis (`self.Axis`))
  (bind _screen_x (`self.Screen X`))
  (`self.Get Screen Pos`)
  ;[1 1 1] 올빼미가 경계를 넘어서게 되면 [ Dir X ] 를 0으로 세팅하여 이동하지 못하게 막는다.
  (if (or (and (< _axis 0.0) (< _screen_x 80.0)) (and (> _axis 0.0) (> _screen_x (- (`self.Screen Width`) 80.0))))
    (set `self.Dir X` 0.0)))

(fn `Get Screen Pos`
  (bind (_x _y) (`KismetMathLibrary.BreakVector2D` (`PlayerController.ProjectWorldLocationToScreen` (`GameplayStatics.GetPlayerController` 0) (`self.K2_GetActorLocation`) false)))
  (set `self.Screen X` _x)
  (set `self.Screen Y` _y))

(fn `Get Screen Size`
  (bind (_sizex _sizey) (`PlayerController.GetViewportSize` (`GameplayStatics.GetPlayerController` 0)))
  (set `self.Screen Width` (`KismetMathLibrary.Conv_IntToDouble` _sizex))
  (set `self.Screen Height` (`KismetMathLibrary.Conv_IntToDouble` _sizey))
  (`KismetSystemLibrary.PrintString` "Get Screen Size 호출!!!"))

(fn `Jump Owl`
  (set `self.Dir Z` (`self.Speed Jump`))
  (`GameplayStatics.PlaySoundAtLocation` "/Game/Audios/jump.jump" (`self.K2_GetActorLocation`) (struct) 1.0 1.0 0.0 null null null))

(fn `Line Interp`
  (params (`Axis Value` :type "Float (double-precision)"))
  (bind _output_get (set `self.Axis` `Axis Value`))
  (set `self.Dir X` (`KismetMathLibrary.FInterpTo` (`self.Dir X`) (* _output_get (`self.Speed Move`)) (`GameplayStatics.GetWorldDeltaSeconds`) 6.0))
  (`self.Check Screen Limit`))

(fn `Move Owl`
  ;[1 1 1] -	올빼미의 상하 이동 속도 = 이전 올빼미의 상하 이동 속도 - 중력 * 프레임 간격 시간.
  ; 	-	[ DirZ ] = [ DirZ ] - [ Gravity ] * [ Get World Delta Seconds ]
  ;
  ; -	해당 함수가 매프레임 호출되면서 [ DirZ ] 값은 0보다 작아져서 아래로 이동하게 될 것.
  (bind _output_get (set `self.Dir Z` (- (`self.Dir Z`) (* (`self.Gravity`) (`GameplayStatics.GetWorldDeltaSeconds`)))))
  (`self.K2_AddActorLocalOffset` (* (`KismetMathLibrary.MakeVector` (`self.Dir X`) 0.0 _output_get) (`GameplayStatics.GetWorldDeltaSeconds`))))

(fn `Set Max Height`
  (bind _z (.z (`self.K2_GetActorLocation`)))
  (if (> _z (`self.Max Height`))
    (set `self.Max Height` _z)))

(fn `UserConstructionScript`)