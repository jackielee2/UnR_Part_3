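; B_Sky is a sky actor that serves as the player's view target and carries an adjustable-speed sky material.
; Its construction script creates a dynamic material instance on the Sky component and feeds SkySpeed into the Speed parameter.
; On BeginPlay it blends the first player controller's view to itself, then calls GetScreenSize on the B_Owl pawn if the cast succeeds.
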(event `self.ReceiveBeginPlay`
  (`PlayerController.SetViewTargetWithBlend` (`GameplayStatics.GetPlayerController` 0) self 0.0 "VTBlend_Linear" 0.0 false)
  (bind _asb_owl (cast `/Game/Blueprints/B_Owl` (`GameplayStatics.GetPlayerPawn` 0)))
  (`/Game/Blueprints/B_Owl.Get Screen Size` _asb_owl))

(fn `UserConstructionScript`
  (bind _returnvalue (`PrimitiveComponent.CreateDynamicMaterialInstance` (`self.Sky`) 0 null "None"))
  (`MaterialInstanceDynamic.SetScalarParameterValue` _returnvalue "Speed" (`self.SkySpeed`)))