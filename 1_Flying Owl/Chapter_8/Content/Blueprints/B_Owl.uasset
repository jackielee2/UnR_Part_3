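; B_Owl is the player owl in a vertical jumper, bouncing off branches while steered horizontally.
; Each Tick traces down for BRANCH-tagged actors to trigger a jump with sound, then applies manual gravity and moves by offset without sweep.
; MoveRight input eases horizontal speed with FInterpTo, zeroing it near screen edges using projected screen position and viewport size refreshed per call.
; New height records are passed to B_Sky to set the camera position.
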(event `self.ReceiveBeginPlay`
  (bind _outactors (`GameplayStatics.GetAllActorsOfClass` "/Game/Blueprints/B_Sky.B_Sky_C")) ; -  맵에 존재하는 특정 클래스( Actor Class )의 모든 액터를 찾아 [ Out Actors ]에 전달.\n     -  연산량이 많으므로 매 프레임( 예 : Tick 이벤트 등.. )마다 호출 지양..
  (set `self.Sky` (`|GetArrayItem` _outactors)))

(event `self.ReceiveTick`
  (params (DeltaSeconds :type "Float (single-precision)"))
  (`self.Check Branch`)
  (`self.Move Owl`)
  (`self.Set Max Height`))

(event `InputAxis|MoveRight`
  (params (AxisValue :type "Float (single-precision)"))
  (`self.Line Interp` AxisValue)
  (`self.Get Screen Size`) ; -  동작할때 마다 화면 크기 얻기.\n\n	-	이전 버전에서 게임 로딩 초기에 화면 크기를 얻었을때\n			PC 에서는 정상 작동하지만 모바일에서는 예상처럼 작동하지 않았음.( 언리얼 버그?? )\n\n	-	키 입력 이벤트가 발생할때마다 크기를 구하므로 상대적으로 자원 낭비 발생.\n			그러나 퍼포먼스 하락을 걱정할 정도는 아님.
)

(fn `Check Branch`
  (bind _returnvalue (`self.K2_GetActorLocation`))
  (bind (_outhit _returnvalue_2) (`KismetSystemLibrary.LineTraceSingle` :`Start` _returnvalue :`End` (+ _returnvalue (0.0 0.0 -40.0)) :`TraceChannel` "TraceTypeQuery3" :`DrawDebugType` "ForOneFrame"))
  (if _returnvalue_2
    (if (`self.ActorHasTag` (`.HitActor` (`GameplayStatics.BreakHitResult` _outhit)) "BRANCH")
      (`self.Jump Owl`))))

(fn `Check Screen Limit`
  (bind _axis (`self.Axis`))
  (bind _screen_x (`self.Screen X`))
  (`self.Get Screen Pos`)
  (if (or (and (< _axis 0.0) (< _screen_x 80.0)) (and (> _axis 0.0) (> _screen_x (- (`self.Screen Width`) 80.0))))
    (set `self.Dir X` 0.0)))

(fn `Get Screen Pos`
  (bind (_x _y) (`KismetMathLibrary.BreakVector2D` (`PlayerController.ProjectWorldLocationToScreen` (`GameplayStatics.GetPlayerController` 0) (`self.K2_GetActorLocation`) false)))
  (set `self.Screen X` _x)
  (set `self.Screen Y` _y))

(fn `Get Screen Size`
  (bind (_sizex _sizey) (`PlayerController.GetViewportSize` (`GameplayStatics.GetPlayerController` 0)))
  (set `self.Screen Width` (`KismetMathLibrary.Conv_IntToDouble` _sizex))
  (set `self.Screen Height` (`KismetMathLibrary.Conv_IntToDouble` _sizey)))

(fn `Jump Owl`
  (set `self.Dir Z` (`self.Speed Jump`))
  (`AudioComponent.Play` (`self.Jump Sound`) 0.01))

(fn `Line Interp`
  (params (`Axis Value` :type "Float (double-precision)"))
  (bind _output_get (set `self.Axis` `Axis Value`))
  (set `self.Dir X` (`KismetMathLibrary.FInterpTo` (`self.Dir X`) (* _output_get (`self.Speed Move`)) (`GameplayStatics.GetWorldDeltaSeconds`) 6.0))
  (`self.Check Screen Limit`))

(fn `Move Owl`
  (bind _output_get (set `self.Dir Z` (- (`self.Dir Z`) (* (`self.Gravity`) (`GameplayStatics.GetWorldDeltaSeconds`)))))
  (`self.K2_AddActorLocalOffset` (* (`KismetMathLibrary.MakeVector` (`self.Dir X`) 0.0 _output_get) (`GameplayStatics.GetWorldDeltaSeconds`))))

(fn `Set Max Height`
  (bind _z (.z (`self.K2_GetActorLocation`)))
  (if (> _z (`self.Max Height`))
    (bind _output_get (set `self.Max Height` _z))
    (`/Game/Blueprints/B_Sky.Set Camera Pos` (`self.Sky`) _output_get)))

(fn `UserConstructionScript`)