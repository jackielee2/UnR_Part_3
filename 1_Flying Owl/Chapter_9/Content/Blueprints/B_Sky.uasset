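; B_Sky is the sky backdrop and view target for a vertical owl game, spawning branches as the view climbs.
; SetCameraPos sets the actor's Z below a supplied max height, while a dynamic material instance applies SkySpeed to the sky.
; BeginPlay spawns the first branch at SpawnPoint.
; Tick adds a randomly X-offset, sized branch whenever SpawnPoint rises more than a fixed gap above the last one.
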(event `self.ReceiveBeginPlay`
  (`PlayerController.SetViewTargetWithBlend` (`GameplayStatics.GetPlayerController` 0) self 0.0 "VTBlend_Linear" 0.0 false)
  (bind _asb_owl (cast `/Game/Blueprints/B_Owl` (`GameplayStatics.GetPlayerPawn` 0)))
  (`/Game/Blueprints/B_Owl.Get Screen Size` _asb_owl)
  (bind _returnvalue (`|SpawnActorFromClass` "/Game/Blueprints/B_Branch.B_Branch_C" (`SceneComponent.K2_GetComponentToWorld` (`self.Spawn Point`)) "Undefined" "OverrideRootScale" null null)) ; - [ Class ]에 설정된 [ 블루프린트 ]를 참고로하여 액터 생성.\n \n -  주요 속성\n     -  [ Class ] : 생성할 액터의 블루프린트 클래스..\n         -  [ B_Branch ]\n     -  [ Spawn Transform ] :  생성할때 참고할 [ 트랜스폼  ]정보.\n         -  [ Spawn Point ] > [ Get World Transform ]
  (set `self.Last Branch` _returnvalue) ; -  [ Spawn actor from class ] > [ Return Value ]를 드래그하여 [ 변수로 승격 ]\n -  추후 생성된 나무가지 액터를 활용하여 새로운 나무가지를 생성할 것 임.
)

(event `self.ReceiveTick`
  (params (DeltaSeconds :type "Float (single-precision)"))
  (`self.Make New Branch`))

(fn `Check New Branch`
  (returns (`Can Branch` :type Boolean) (Location :type "Vector Structure"))
  (bind _returnvalue (> (.z (`SceneComponent.K2_GetComponentLocation` (`self.Spawn Point`))) (+ (.z (`self.K2_GetActorLocation` (`self.Last Branch`))) 300.0)))
  ;[1 1 1] 3)  1) > 2) 인지 체크후
  ;    - [ T ]  :  [ Get Branch Location ] 처리후
  ;                   나무가지가 새로 생성될 위치값과 체크 결과 반환.
  ;
  ;    - [ F ]  :  [ Location ]에 데이터가 전달되지 않으므로
  ;                   기본값[ 0, 0, 0]과 체크 결과만 반환.
  (if _returnvalue
    (bind _return_value (`self.Get Branch Location`)))
  (return _returnvalue _return_value))

(fn `Get Branch Location`
  (returns (`Return Value` :type "Vector Structure"))
  (return (`KismetMathLibrary.MakeVector` (`KismetMathLibrary.RandomFloatInRange` -250.0 250.0) (.y (`SceneComponent.K2_GetComponentLocation` (`self.Spawn Point`))) (.z (`SceneComponent.K2_GetComponentLocation` (`self.Spawn Point`))))))

(fn `Make New Branch`
  (bind (_can_branch _location) (`self.Check New Branch`)) ; 1)  새로운 나뭇가지가 필요한지 조사후 필요한 경우에만 이하 처리..
  (if _can_branch
    ;[1 1 1] 2)  나무가지 생성
    (bind _returnvalue (`|SpawnActorFromClass` "/Game/Blueprints/B_Branch.B_Branch_C" (`KismetMathLibrary.Conv_VectorToTransform` _location) "Undefined" "OverrideRootScale" null null))
    (bind _output_get (set `self.Last Branch` _returnvalue))
    (`/Game/Blueprints/B_Branch.Set Branch Size` _output_get) ; 3)  나무가지 사이즈 설정..
  ))

(fn `Set Camera Pos`
  (params (`Max Height` :type "Float (double-precision)"))
  (`self.K2_SetActorLocation` (`KismetMathLibrary.MakeVector` 0.0 0.0 (- `Max Height` 320.0))))

(fn `UserConstructionScript`
  (bind _returnvalue (`PrimitiveComponent.CreateDynamicMaterialInstance` (`self.Sky`) 0 null "None"))
  (`MaterialInstanceDynamic.SetScalarParameterValue` _returnvalue "Speed" (`self.SkySpeed`)))