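; BP_Light is a light actor that switches on when its Box trigger is first overlapped and registers itself as an active light.
; The overlap passes through a DoOnce, sets IsLightOn, then increments NumbersOfActiveLights on BP_MyGameMode and prints the count.
; Tick applies IsLightOn to the PointLight's visibility every frame.
; The overlapping actor is not filtered, and nothing here switches the light off.
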(event `self.Box.OnComponentBeginOverlap`
  (params (OverlappedComponent :type "PrimitiveComponent Object Reference") (OtherActor :type "Actor Object Reference") (OtherComp :type "PrimitiveComponent Object Reference") (OtherBodyIndex :type Integer) (bFromSweep :type Boolean) (SweepResult :type "HitResult Structure (by ref)"))
  (`/Engine/EditorBlueprintResources/StandardMacros.DoOnce` false ; 1) 처음 한 번만 이 노드 다음에 연결된 노드를 처리하고 그 이후에는 처리하지 않음.\n     - 이미 활성화된 조명에 다시 캐릭터가 충돌하더라도 카운팅 되지 않도록 처리하기 위해 사용.
    (:`Completed`
      (set `self.Is Light On` true)
      (bind _asbp_my_game_mode (cast `/Game/Cute_Girl/Blueprints/BP_MyGameMode` (`GameplayStatics.GetGameMode`))) ; 3) [ Game Mode Base ]를 [ BP_MyGameMode ]로 형변환
      ;[1 1 1] 4) 활성화된 조명수 카운트 + 1
      (bind _result (`/Engine/EditorBlueprintResources/StandardMacros.IncrementInt` (`/Game/Cute_Girl/Blueprints/BP_MyGameMode.Numbers of Active Lights` _asbp_my_game_mode))
        (:`  `
          (`KismetSystemLibrary.PrintString` (`KismetStringLibrary.Conv_IntToString` _result)) ; 5) 컴파일 후 테스트
        )))))

(event `self.ReceiveTick`
  (params (DeltaSeconds :type "Float (single-precision)"))
  (`SceneComponent.SetVisibility` (`self.PointLight`) (`self.Is Light On`) false) ; 1) 액터의 가시성 설정
)

(fn `UserConstructionScript`)