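; BP_Character is a player character with movement, jumping, health and a game-over trigger.
; Movement inputs follow control yaw, scaled by a Speed value that Left Shift raises while held.
; AnyDamage briefly swaps a body material as a hit flash and subtracts from Health.
; When Health runs out, GameOver casts to BP_MyGameMode and reports a failed result through GameResult.
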(event `Damaged`
  (`KismetSystemLibrary.PrintString` "Damaged!!!"))

(event `self.ReceiveAnyDamage`
  (params (Damage :type "Float (single-precision)") (DamageType :type "DamageType Object Reference") (InstigatedBy :type "Controller Object Reference") (DamageCauser :type "Actor Object Reference"))
  (bind _health (`self.Health`))
  (`self.Damage Body`) ; 대미지 이펙트 연출
  ;[1 1 1] 2)  [ Health ]가 0이하라면 처리
  (if (<= _health 0.0)
    (`KismetSystemLibrary.PrintString` "You are already Dead!!!")
    (else
      ;[1 1 1] 3)  [ Health ]가 0보다 크면 [ Health ]에 대미지를 차감
      (bind _output_get (set `self.Health` (- _health Damage)))
      (`KismetSystemLibrary.PrintString` (`KismetStringLibrary.Conv_DoubleToString` _output_get))
      ;[1 1 1] 4)  [ Health ] <= 0  인 경우
      ;       "Dead" 출력
      (if (<= _output_get 0.0)
        (`self.Game Over`)))))

(event `InputAxis|MoveForward`
  (params (AxisValue :type "Float (single-precision)"))
  ;[1 1 1] 이동
  (`self.AddMovementInput` (`KismetMathLibrary.GetForwardVector` (`KismetMathLibrary.MakeRotator` 0.0 0.0 (.yaw (`self.GetControlRotation`)))) (* AxisValue (`self.Speed`))))

(event `Key|LeftShift`
  (params (Key :type "Key Structure"))
  ;[1 1 1] 부스트
  (:`Pressed`
    (set `self.Speed` 1.0))
  (:`Released`
    (set `self.Speed` 0.5)))

(event `InputAxis|MoveRight`
  (params (AxisValue :type "Float (single-precision)"))
  ;[1 1 1] 이동
  (`self.AddMovementInput` (`KismetMathLibrary.GetRightVector` (`KismetMathLibrary.MakeRotator` 0.0 0.0 (.yaw (`self.GetControlRotation`)))) (* AxisValue (`self.Speed`))))

(event `InputAction|Jump`
  (params (Key :type "Key Structure"))
  ;[1 1 1] 점프
  (:`Pressed`
    (`self.Jump`) ; 2) [ Character / Jump 함수 ]
  ))

(event `Damage Body`
  (bind _mesh (`self.Mesh`))
  (`PrimitiveComponent.SetMaterial` _mesh 2 "/Game/Cute_Girl/Materials/DamagedMaterial.DamagedMaterial") ; 1) 타깃 메시에 특정 머터리얼 설정\n   - 머터리얼 엘리먼트 2에 [ DamagedMaterial  ] 연결
  (`KismetSystemLibrary.Delay` 0.2) ; 2)  다음 노드를 처리하기전에 일정시간 대기
  (`PrimitiveComponent.SetMaterial` _mesh 2 "/Game/Cute_Girl/Materials/T_Liz_Body_Mat.T_Liz_Body_Mat") ; 3)  원래 머터리얼로 리셋\n     -  이전 [ Set Material ]에 [ Mesh ]노드가 있으므로\n         재사용한다
)

(event `Game Over`
  (bind _asbp_my_game_mode (cast `/Game/Cute_Girl/Blueprints/BP_MyGameMode` (`GameplayStatics.GetGameMode`))) ; 1)  [ BP_MyGameMode ] 연결.\n      -  [ BP_MyGameMode ] > [ Game Result ]를 호출하기 위해..
  (`/Game/Cute_Girl/Blueprints/BP_MyGameMode.Game Result` _asbp_my_game_mode false) ; 2)  [ Clear 입력 핀 ]  :  체크해제\n     - [ Game Result ] > [ Clear ]에 False 값이 전달되어 [ GameOver ] 화면 표시
)

(fn `UserConstructionScript`)