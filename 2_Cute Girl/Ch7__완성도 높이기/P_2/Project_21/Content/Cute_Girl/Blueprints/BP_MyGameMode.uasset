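; Game mode that shows the player HUD, tracks score and light activation, and displays the end-of-game screen.
; Every Tick it recounts BP_Light actors and sets IsExploding, the bomb trigger, when that total equals NumbersOfActiveLights, which is not modified here.
; AddScore counts collected items and calls GameResult with a clear once five are reached.
; GameResult creates either ClearUI or GameOverUI from its Clear flag and adds it to the viewport.
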(event `self.ReceiveBeginPlay`
  (bind _returnvalue (`GameplayStatics.GetPlayerController` 0))
  (bind _returnvalue_2 (`|CreateWidget` "/Game/Cute_Girl/UMG/PlayerUI.PlayerUI_C")) ; 1) [ 위젯 생성  ] 검색 및 추가\n     - [ Class ]   :   PlayerUI
  (`UserWidget.AddToViewport` _returnvalue_2 0) ; 2) 게임화면에 위젯을 표시하기 위한 노드.
  (`/Engine/EditorBlueprintResources/StandardMacros.IsValid` _returnvalue
    (:`Is Valid`
      (`WidgetBlueprintLibrary.SetInputMode_GameOnly` _returnvalue))))

(event `self.ReceiveTick`
  (params (DeltaSeconds :type "Float (single-precision)"))
  ;[1 1 1] 3) 현재 레벨에 설치된 조명의 갯수를 Numbers of Lights에 설정
  (bind _outactors (`GameplayStatics.GetAllActorsOfClass` "/Game/Cute_Girl/Blueprints/BP_Light.BP_Light_C")) ; 1) 같은 레벨에 있는 특정 클래스의 모든 액터를 배열로 참조.    [ Actor Class ] : BP_Light
  (bind _output_get (set `self.Numbers of Lights` (`KismetArrayLibrary.Array_Length` _outactors)))
  ;[1 1 1] 4) 활성화된 조명의 갯수와 설치된 조명의 갯수가 같다면 폭탄을 터뜨리도록 설정.
  (if (== _output_get (`self.Numbers of Active Lights`))
    (set `self.Is Exploding` true)))

(event `Game Result`
  (params (Clear :type Boolean))
  (bind _returnvalue (`|CreateWidget` (select `bool` Clear :`false` "/Game/Cute_Girl/UMG/GameOverUI.GameOverUI_C" :`true` "/Game/Cute_Girl/UMG/ClearUI.ClearUI_C" :!type "UserWidget Class Reference"))) ; 2)  [ 위젯 생성 ] 검색 후 선택\n     - [ Class 입력 핀 ]이 설정되지 않아 [ NONE 생성 ]으로 표시.
  (`UserWidget.AddToViewport` _returnvalue 0) ; 5) 위젯을 화면에 표시
)

(fn `Add Score`
  ;[1 1 1] 1) [ Total Score ]의 값에 1을 누적..
  (bind _result (`/Engine/EditorBlueprintResources/StandardMacros.IncrementInt` (`self.Total Score`))
    (:`  `
      ;[1 1 1] 2)  아이템 획득수가 5개 이상인 경우 Clear 처리
      (if (>= _result 5)
        (`self.Game Result` true)))))

(fn `UserConstructionScript`)