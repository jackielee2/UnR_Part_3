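; BP_TestActor_2 is a test actor that logs its own variables when play begins.
; On BeginPlay it prints its integer, float, boolean and string variables in sequence, converting the non-string ones to text.
; Overlap, Tick and the construction script are empty.
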(event `self.ReceiveBeginPlay`
  (`KismetSystemLibrary.PrintString` (`KismetStringLibrary.Conv_IntToString` (`self.Int Test`)))
  (`KismetSystemLibrary.PrintString` (`KismetStringLibrary.Conv_DoubleToString` (`self.float Test`)))
  (`KismetSystemLibrary.PrintString` (`KismetStringLibrary.Conv_BoolToString` (`self.bool Test`)))
  (`KismetSystemLibrary.PrintString` (`self.string Test`)))

(fn `UserConstructionScript`)