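; BP_MinMaxMulti is a quiz practice actor that prints every multiple of a given number within a range.
; On BeginPlay it passes its Min, Max and Multi variables to the ShowMulti function.
; ShowMulti loops from Min to Max and prints each index whose remainder modulo Multi is zero.
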(event `self.ReceiveBeginPlay`
  (`self.Show_Multi` (`self.min`) (`self.max`) (`self.multi`)))

(fn `Show_Multi`
  (params (min :type Integer) (max :type Integer) (multi :type Integer))
  (for _index (range min (+ max 1))
    (if (== (mod _index multi) 0)
      (`KismetSystemLibrary.PrintString` (`KismetStringLibrary.Conv_IntToString` _index)))))

(fn `UserConstructionScript`)