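; BP_Enemy_3 is a shooting-game enemy that flies in a straight line at constant speed.
; On BeginPlay, a random roll against TraceRate aims it either at the BP_Player_9 actor's current position or along its own forward vector.
; Tick moves it along that stored direction by MoveSpeed scaled with delta time, without sweeping, so it never re-aims.
; The overlap event is an empty stub.
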(event `self.ReceiveBeginPlay`
  (if (<= (`KismetMathLibrary.RandomFloatInRange` 0.0 1.0) (`self.Trace Rate`))
    (bind _returnvalue (`GameplayStatics.GetActorOfClass` "/Game/Shooting_Game_BP/Lesson_12/BP/BP_Player_9.BP_Player_9_C"))
    (set `self.Dir` (`KismetMathLibrary.Normal` (- (`self.K2_GetActorLocation` _returnvalue) (`self.K2_GetActorLocation`))))
    (else
      (set `self.Dir` (`self.GetActorForwardVector`)))))

(event `self.ReceiveTick`
  (params (DeltaSeconds :type "Float (single-precision)"))
  (`self.K2_SetActorLocation` (+ (`self.K2_GetActorLocation`) (* (* (`self.Dir`) (`self.Move Speed`)) DeltaSeconds))))

(fn `UserConstructionScript`)