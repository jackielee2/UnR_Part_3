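; BP_Bullet_4 is a shooting-game projectile that destroys enemies it touches.
; Tick moves it along its forward vector at MoveSpeed, scaled by DeltaSeconds, using a non-swept location update.
; On actor overlap with a BP_Enemy_5, it destroys that enemy, spawns the P_Explosion emitter at its own location, then destroys itself.
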(event `self.ReceiveTick`
  (params (DeltaSeconds :type "Float (single-precision)"))
  (`self.K2_SetActorLocation` (+ (`self.K2_GetActorLocation`) (* (* (`self.GetActorForwardVector`) (`self.MoveSpeed`)) DeltaSeconds))))

(event `self.ReceiveActorBeginOverlap`
  (params (OtherActor :type "Actor Object Reference"))
  (bind _asbp_enemy_5 (cast `/Game/Shooting_Game_BP/Lesson_17/BP/BP_Enemy_5` OtherActor))
  (`self.K2_DestroyActor` _asbp_enemy_5)
  (`GameplayStatics.SpawnEmitterAtLocation` "/Game/StarterContent/Particles/P_Explosion.P_Explosion" (`self.K2_GetActorLocation`))
  (`self.K2_DestroyActor`))

(fn `UserConstructionScript`)