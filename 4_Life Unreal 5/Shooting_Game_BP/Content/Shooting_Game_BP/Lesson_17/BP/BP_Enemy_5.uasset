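; BP_Enemy_5 is a shooting-game enemy that flies in a straight line and destroys the player on contact.
; On BeginPlay, a random roll against TraceRate either aims it once at BP_Player_12's current location, rotating it to face that way, or keeps its forward vector.
; Tick moves it along that fixed direction at MoveSpeed without sweeping.
; Overlapping the player destroys both actors and spawns an explosion at the enemy's location.
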(event `self.ReceiveBeginPlay`
  (if (<= (`KismetMathLibrary.RandomFloatInRange` 0.0 1.0) (`self.Trace Rate`))
    (bind _returnvalue (`GameplayStatics.GetActorOfClass` "/Game/Shooting_Game_BP/Lesson_17/BP/BP_Player_12.BP_Player_12_C"))
    (`/Engine/EditorBlueprintResources/StandardMacros.IsValid` _returnvalue
      (:`Is Valid`
        (bind _output_get (set `self.Dir` (`KismetMathLibrary.Normal` (- (`self.K2_GetActorLocation` _returnvalue) (`self.K2_GetActorLocation`)))))
        (`self.K2_SetActorRotation` (`KismetMathLibrary.MakeRotFromXZ` _output_get (`self.GetActorUpVector`)))))
    (else
      (set `self.Dir` (`self.GetActorForwardVector`)))))

(event `self.ReceiveTick`
  (params (DeltaSeconds :type "Float (single-precision)"))
  (`self.K2_SetActorLocation` (+ (`self.K2_GetActorLocation`) (* (* (`self.Dir`) (`self.Move Speed`)) DeltaSeconds))))

(event `self.ReceiveActorBeginOverlap`
  (params (OtherActor :type "Actor Object Reference"))
  (bind _asbp_player_12 (cast `/Game/Shooting_Game_BP/Lesson_17/BP/BP_Player_12` OtherActor))
  (`self.K2_DestroyActor` _asbp_player_12)
  (`GameplayStatics.SpawnEmitterAtLocation` "/Game/StarterContent/Particles/P_Explosion.P_Explosion" (`self.K2_GetActorLocation`))
  (`self.K2_DestroyActor`))

(fn `UserConstructionScript`)