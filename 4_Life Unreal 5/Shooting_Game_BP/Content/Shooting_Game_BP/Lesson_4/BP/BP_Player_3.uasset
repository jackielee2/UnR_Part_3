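; BP_Player_3 is a player Blueprint for a shooting game lesson that captures horizontal and vertical input without applying it to movement.
; BeginPlay adds the IMC_PlayerInput_2 mapping context to player 0's Enhanced Input subsystem.
; The IA_Horizontal and IA_Vertical actions store their values in Horizontal and Vertical on Triggered and Completed, printing each for debugging.
; Tick, overlap and construction logic are empty.
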(event `self.ReceiveBeginPlay`
  (`EnhancedInputSubsystemInterface.AddMappingContext` (pcsubsystem `EnhancedInputLocalPlayerSubsystem` (`GameplayStatics.GetPlayerController` 0)) "/Game/Shooting_Game_BP/Lesson_3_2/Inputs/IMC_PlayerInput_2.IMC_PlayerInput_2" 0 (struct)))

(event `EnhancedInput|/Game/Shooting_Game_BP/Lesson_2/Inputs/IA_Horizontal`
  (params (ActionValue :type "Float (double-precision)") (ElapsedSeconds :type "Float (double-precision)") (TriggeredSeconds :type "Float (double-precision)") (InputAction :type "InputAction Object Reference" :default "/Game/Shooting_Game_BP/Lesson_2/Inputs/IA_Horizontal.IA_Horizontal"))
  (:`Triggered`
    (bind _output_get (set `self.Horizontal` ActionValue))
    (`KismetSystemLibrary.PrintString` (`KismetStringLibrary.Concat_StrStr` "Horzontal : " (`KismetStringLibrary.Conv_DoubleToString` _output_get))))
  (:`Completed`
    (bind _output_get_2 (set `self.Horizontal` ActionValue))
    (`KismetSystemLibrary.PrintString` (`KismetStringLibrary.Concat_StrStr` "Horzontal : " (`KismetStringLibrary.Conv_DoubleToString` _output_get_2)))))

(event `EnhancedInput|/Game/Shooting_Game_BP/Lesson_3_2/Inputs/IA_Vertical`
  (params (ActionValue :type "Float (double-precision)") (ElapsedSeconds :type "Float (double-precision)") (TriggeredSeconds :type "Float (double-precision)") (InputAction :type "InputAction Object Reference" :default "/Game/Shooting_Game_BP/Lesson_3_2/Inputs/IA_Vertical.IA_Vertical"))
  (:`Triggered`
    (bind _output_get (set `self.Vertical` ActionValue))
    (`KismetSystemLibrary.PrintString` (`KismetStringLibrary.Concat_StrStr` "Vertical : " (`KismetStringLibrary.Conv_DoubleToString` _output_get))))
  (:`Completed`
    (bind _output_get_2 (set `self.Vertical` ActionValue))
    (`KismetSystemLibrary.PrintString` (`KismetStringLibrary.Concat_StrStr` "Vertical : " (`KismetStringLibrary.Conv_DoubleToString` _output_get_2)))))

(fn `UserConstructionScript`)