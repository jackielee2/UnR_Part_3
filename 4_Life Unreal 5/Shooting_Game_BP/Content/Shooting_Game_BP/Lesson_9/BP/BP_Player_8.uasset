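; Player pawn for a shooting game lesson that moves on the Y-Z plane and fires bullets.
; BeginPlay adds an Enhanced Input mapping context, and horizontal and vertical actions store their axis values on trigger and completion.
; Tick normalizes those axes into a direction, scales it by MoveSpeed and delta time, and sets the location without sweep.
; The fire action spawns BP_Bullet at the FirePosition component's transform.
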(event `self.ReceiveBeginPlay`
  (`EnhancedInputSubsystemInterface.AddMappingContext` (pcsubsystem `EnhancedInputLocalPlayerSubsystem` (`GameplayStatics.GetPlayerController` 0)) "/Game/Shooting_Game_BP/Lesson_9/Inputs/IMC_PlayerInput_3.IMC_PlayerInput_3" 0 (struct)))

(event `EnhancedInput|/Game/Shooting_Game_BP/Lesson_2/Inputs/IA_Horizontal`
  (params (ActionValue :type "Float (double-precision)") (ElapsedSeconds :type "Float (double-precision)") (TriggeredSeconds :type "Float (double-precision)") (InputAction :type "InputAction Object Reference" :default "/Game/Shooting_Game_BP/Lesson_2/Inputs/IA_Horizontal.IA_Horizontal"))
  (:`Triggered`
    (set `self.Horizontal` ActionValue))
  (:`Completed`
    (set `self.Horizontal` ActionValue)))

(event `self.ReceiveTick`
  (params (DeltaSeconds :type "Float (single-precision)"))
  (`self.K2_SetActorLocation` (+ (`self.K2_GetActorLocation`) (* (* (`KismetMathLibrary.Normal` (`KismetMathLibrary.MakeVector` 0.0 (`self.Horizontal`) (`self.Vertical`))) (`self.MoveSpeed`)) DeltaSeconds))))

(event `EnhancedInput|/Game/Shooting_Game_BP/Lesson_3_2/Inputs/IA_Vertical`
  (params (ActionValue :type "Float (double-precision)") (ElapsedSeconds :type "Float (double-precision)") (TriggeredSeconds :type "Float (double-precision)") (InputAction :type "InputAction Object Reference" :default "/Game/Shooting_Game_BP/Lesson_3_2/Inputs/IA_Vertical.IA_Vertical"))
  (:`Triggered`
    (set `self.Vertical` ActionValue))
  (:`Completed`
    (set `self.Vertical` ActionValue)))

(event `EnhancedInput|/Game/Shooting_Game_BP/Lesson_9/Inputs/IA_Fire`
  (params (ActionValue :type Boolean) (ElapsedSeconds :type "Float (double-precision)") (TriggeredSeconds :type "Float (double-precision)") (InputAction :type "InputAction Object Reference" :default "/Game/Shooting_Game_BP/Lesson_9/Inputs/IA_Fire.IA_Fire"))
  (:`Started`
    (`|SpawnActorFromClass` "/Game/Shooting_Game_BP/Lesson_8/BP/BP_Bullet.BP_Bullet_C" (`SceneComponent.K2_GetComponentToWorld` (`self.Fire Position`)) "AlwaysSpawn" "MultiplyWithRoot" null null)))

(fn `UserConstructionScript`)